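; Game instance hub that creates and shows the menu, HUD, pause, loading and level-completion widgets, and handles returning to menu and restarting levels.
; The selected map index and Timer or Record type drive restarts and results.
; On a win, HUD time and score are merged with stored bests and time-threshold stars, then written to one save slot.
; UpdateMapSlotInst creates or loads that save and caches its map array for lookups.
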(event `Show Main Menu`
  (bind _returnvalue (`GameplayStatics.GetPlayerController` 0))
  ;[1 1 1] Запуск главного меню (из левел блупринта)
  (`/Engine/EditorBlueprintResources/StandardMacros.IsValid` (`self.Main Menu WB`)
    (:`Is Valid`
      _)
    (:`Is Not Valid`
      (bind _returnvalue_2 (`|CreateWidget` "/Game/2Maps/MainMenu/MainMenu_WB.MainMenu_WB_C"))
      (bind _output_get (set `self.Main Menu WB` _returnvalue_2))))
  (`UserWidget.AddToViewport` _output_get 0)
  (set `PlayerController.bShowMouseCursor` true _returnvalue)
  (`WidgetBlueprintLibrary.SetInputMode_UIOnlyEx` _returnvalue (`self.Main Menu WB`)))

(event `Show Maps Menu`
  ;[1 1 1] Открыть меню карт
  (`/Engine/EditorBlueprintResources/StandardMacros.IsValid` (`self.Map Memu WB`)
    (:`Is Valid`
      _)
    (:`Is Not Valid`
      (bind _returnvalue (`|CreateWidget` "/Game/2Maps/MainMenu/MM_Map_WB.MM_Map_WB_C"))
      (bind _output_get (set `self.Map Memu WB` _returnvalue))))
  (`UserWidget.AddToViewport` _output_get 0))

(event `Player Loaded`
  ;[1 1 1] Игрок загрузился
  (`/Engine/EditorBlueprintResources/StandardMacros.IsValid` (`self.HUD WB`)
    (:`Is Valid`
      _)
    (:`Is Not Valid`
      (bind _returnvalue (`|CreateWidget` "/Game/7Wiget/HUD/HUD_WB.HUD_WB_C"))
      (bind _output_get (set `self.HUD WB` _returnvalue))))
  (`UserWidget.AddToViewport` _output_get 0))

(event `Save Game to Slot`
  (params (Stars :type Integer) (`Best Time` :type Integer) (`Best Score` :type Integer))
  ;[1 0.8808 0.185] Сохранение игры *Ред*
  (set `self.Stars` Stars)
  (set `self.BestTime` `Best Time`)
  (set `self.Best Score` `Best Score`)
  (bind _returnvalue (`GameplayStatics.DoesSaveGameExist` "SaveGame1"))
  (if _returnvalue
    (bind _returnvalue_2 (`GameplayStatics.LoadGameFromSlot` "SaveGame1"))
    (bind _assave_game_bp (cast `/Game/5Save/SaveGame_BP` _returnvalue_2))
    (bind (_mapindex _namemap _imagemap _starscomplete _besttime _score _stars1time _stars2time _stars3time _systemnamemaptime _systemnamemaprecord _systempage _systemleveltype) (break `/Game/5Save/S_MapSlot_Info` (`|GetArrayItem` (`/Game/5Save/SaveGame_BP.Save Game Slot S Array` _assave_game_bp) (`self.MapPlayedNow Index`))))
    (`KismetArrayLibrary.Array_Set` (`/Game/5Save/SaveGame_BP.Save Game Slot S Array` _assave_game_bp) (`self.MapPlayedNow Index`) (make `/Game/5Save/S_MapSlot_Info` _mapindex _namemap _imagemap (`self.Stars`) (`self.BestTime`) (`self.Best Score`) _stars1time _stars2time _stars3time _systemnamemaptime "None" _systempage _systemleveltype))
    (`GameplayStatics.SaveGameToSlot` _assave_game_bp "SaveGame1")))

(event `Delete Save Slot`
  ;[1 0.8808 0.185] Сохранение игры *Ред*
  ;;[1 1 1] Удаление сохранения
  (`GameplayStatics.DeleteGameInSlot` "SaveGame1"))

(event `Update Map Slot Inst`
  ;[1 0.8808 0.185] Сохранение игры *Ред*
  (bind _returnvalue (`GameplayStatics.DoesSaveGameExist` "SaveGame1"))
  (if _returnvalue
    (bind _returnvalue_2 (`GameplayStatics.LoadGameFromSlot` "SaveGame1"))
    (bind _assave_game_bp (cast `/Game/5Save/SaveGame_BP` _returnvalue_2 :!pure true))
    (bind _save_game_slot_s_array (`/Game/5Save/SaveGame_BP.Save Game Slot S Array` _assave_game_bp))
    (set `self.Save Game Slot` _save_game_slot_s_array)
    (for (_array_element _array_index) _save_game_slot_s_array
      (`KismetArrayLibrary.Array_Set` _save_game_slot_s_array _array_index _array_element))
    (`GameplayStatics.SaveGameToSlot` _assave_game_bp "SaveGame1")
    (else
      (bind _returnvalue_3 (`GameplayStatics.CreateSaveGameObject` "/Game/5Save/SaveGame_BP.SaveGame_BP_C"))
      (bind _save_game_slot_s_array_2 (`/Game/5Save/SaveGame_BP.Save Game Slot S Array` _returnvalue_3))
      (set `self.Save Game Slot` _save_game_slot_s_array_2)
      (for (_array_element_2 _array_index_2) _save_game_slot_s_array_2
        (`KismetArrayLibrary.Array_Set` _save_game_slot_s_array_2 _array_index_2 _array_element_2))
      (`GameplayStatics.SaveGameToSlot` _returnvalue_3 "SaveGame1"))))

(event `Open Pause Menu`
  ;[1 1 1] Открыть меню паузы
  (`GameplayStatics.SetGamePaused` true)
  (`/Engine/EditorBlueprintResources/StandardMacros.IsValid` (`self.Pause Menu WB`)
    (:`Is Valid`
      _)
    (:`Is Not Valid`
      (bind _returnvalue (`|CreateWidget` "/Game/7Wiget/PauseMenu_WB.PauseMenu_WB_C"))
      (bind _output_get (set `self.Pause Menu WB` _returnvalue))))
  (`UserWidget.AddToViewport` _output_get 0)
  (`WidgetBlueprintLibrary.SetInputMode_UIOnlyEx` (`GameplayStatics.GetPlayerController` 0) _returnvalue))

(event `Close Pause Menu`
  ;[1 1 1] Закрыть меню паузы
  (`GameplayStatics.SetGamePaused` false)
  (`WidgetBlueprintLibrary.SetInputMode_GameOnly` (`GameplayStatics.GetPlayerController` 0))
  (`/Engine/EditorBlueprintResources/StandardMacros.IsValid` (`self.HUD WB`)
    (:`Is Valid`
      _)
    (:`Is Not Valid`
      (bind _returnvalue (`|CreateWidget` "/Game/7Wiget/HUD/HUD_WB.HUD_WB_C"))
      (bind _output_get (set `self.HUD WB` _returnvalue))))
  (`UserWidget.AddToViewport` _output_get 0))

(event `Go To Main Menu`
  ;[1 1 1] В главное меню
  (`GameplayStatics.SetGamePaused` false)
  (`/Game/7Wiget/HUD/HUD_WB.Clear Time` (`self.HUD WB`))
  (`/Engine/EditorBlueprintResources/StandardMacros.IsValid` (`self.Loading WB`)
    (:`Is Valid`
      _)
    (:`Is Not Valid`
      (bind _returnvalue (`|CreateWidget` "/Game/2Maps/MainMenu/Loading_WB.Loading_WB_C"))
      (bind _output_get (set `self.Loading WB` _returnvalue))))
  (`UserWidget.AddToViewport` _output_get 0)
  (`KismetSystemLibrary.Delay` 1.5)
  (`GameplayStatics.OpenLevel` "MainMenu_Map")
  (`KismetSystemLibrary.Delay` 0.5)
  (`Widget.RemoveFromParent` (`self.Loading WB`)))

(event `Level End`
  (params (`Win?` :type Boolean))
  (bind _hud_wb (`self.HUD WB`))
  (bind _time (`/Game/7Wiget/HUD/HUD_WB.Time` _hud_wb))
  ;[1 1 1] Завершение левела
  (if `Win?`
    (`/Game/7Wiget/HUD/HUD_WB.Stop Time` _hud_wb)
    (`self.Save Game to Slot` (`self.Get Best Stars` _time) (`self.Get Best Time` _time) (`self.Get Best Score` (`/Game/7Wiget/HUD/HUD_WB.Score` _hud_wb)))
    (bind _returnvalue (`|CreateWidget` "/Game/7Wiget/CompleteLevel_WB.CompleteLevel_WB_C" null (`self.Now Level Type`) true))
    (bind _output_get (set `self.Complete Level WB` _returnvalue))
    (`UserWidget.AddToViewport` _output_get 0)
    (`/Game/7Wiget/HUD/HUD_WB.Clear Time` (`self.HUD WB`))
    (else
      (`/Game/7Wiget/HUD/HUD_WB.Stop Time` (`self.HUD WB`))
      (bind _returnvalue_2 (`|CreateWidget` "/Game/7Wiget/CompleteLevel_WB.CompleteLevel_WB_C" null (`self.Now Level Type`)))
      (bind _output_get_2 (set `self.Complete Level WB` _returnvalue_2))
      (`UserWidget.AddToViewport` _output_get_2 0)
      (`/Game/7Wiget/HUD/HUD_WB.Clear Time` (`self.HUD WB`)))))

(event `Add Value to Score`
  (params (`Add Value` :type Integer))
  ;[1 1 1] Добавить значение в счет
  (`/Game/7Wiget/HUD/HUD_WB.Add Score` (`self.HUD WB`) `Add Value`))

(event `Restart Level`
  (bind _hud_wb (`self.HUD WB`))
  (bind (_mapindex _namemap _imagemap _starscomplete _besttime _score _stars1time _stars2time _stars3time _systemnamemaptime _systemnamemaprecord) (break `/Game/5Save/S_MapSlot_Info` (`|GetArrayItem` (`self.Save Game Slot`) (`self.MapPlayedNow Index`))))
  ;[1 1 1] Перезагрузка левела
  (switch `/Game/5Save/E_LevelType` (`self.Now Level Type`)
    (:`NewEnumerator0`
      (`GameplayStatics.OpenLevel` _systemnamemaptime))
    (:`NewEnumerator1`
      (`GameplayStatics.OpenLevel` _systemnamemaprecord)))
  (`WidgetBlueprintLibrary.SetInputMode_GameOnly` (`GameplayStatics.GetPlayerController` 0))
  (`/Game/7Wiget/HUD/HUD_WB.Clear Time` _hud_wb)
  (set `/Game/7Wiget/HUD/HUD_WB.Score` 0 _hud_wb))

(fn `Get Best Score`
  (params (Score :type Integer))
  (returns (`Best Score` :type Integer))
  (locals (`Local Score` :type Integer))
  (bind (_mapindex _namemap _imagemap _starscomplete _besttime _score) (break `/Game/5Save/S_MapSlot_Info` (`|GetArrayItem` (`self.Save Game Slot`) (`self.MapPlayedNow Index`))))
  (set `local.Local Score` Score)
  (if (== _score 0)
    (return (`local.Local Score`))
    (elif (< _score (`local.Local Score`))
      (return (`local.Local Score`))
      (else
        (return _score)))))

(fn `Get Best Stars`
  (params (Time :type Integer))
  (returns (`Best Stars` :type Integer))
  (bind _stars (`self.Get Stars` Time))
  (bind (_mapindex _namemap _imagemap _starscomplete) (break `/Game/5Save/S_MapSlot_Info` (`|GetArrayItem` (`self.Save Game Slot`) (`self.MapPlayedNow Index`))))
  (if (> _stars _starscomplete)
    (return _stars)
    (else
      (return _starscomplete))))

(fn `Get Best Time`
  (params (Time :type Integer))
  (returns (`Best time` :type Integer))
  (bind (_mapindex _namemap _imagemap _starscomplete _besttime) (break `/Game/5Save/S_MapSlot_Info` (`|GetArrayItem` (`self.Save Game Slot`) (`self.MapPlayedNow Index`))))
  (if (== _besttime 0)
    (return Time)
    (elif (< Time _besttime)
      (return Time)
      (else
        (return _besttime)))))

(fn `Get Stars`
  (params (Time :type Integer))
  (returns (Stars :type Integer))
  (bind (_mapindex _namemap _imagemap _starscomplete _besttime _score _stars1time _stars2time _stars3time) (break `/Game/5Save/S_MapSlot_Info` (`|GetArrayItem` (`self.Save Game Slot`) (`self.MapPlayedNow Index`))))
  (if (<= Time _stars3time)
    (return 3)
    (elif (<= Time _stars2time)
      (return 2)
      (elif (<= Time _stars1time)
        (return 1)
        (else
          (return 0))))))

(fn `Set Now Index and Level Type`
  (params (Index :type Integer) (`Level Type` :type "/Game/5Save/E_LevelType Enum" :default "NewEnumerator0"))
  (set `self.MapPlayedNow Index` Index)
  (set `self.Now Level Type` `Level Type`)
  (return))